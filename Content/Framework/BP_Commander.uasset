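; BP_Commander is a camera actor that pans when the cursor nears a viewport edge.
; On BeginPlay it becomes the view target and caches BP_ControllerBase.
; Each Tick it turns mouse position into per-axis steps of -1, 0 or 1 and offsets the root by CameraSpeed, without delta-time scaling.
; Panning runs only while the controller's Direction X and Y are zero, unless CombineMovement is set.
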(event `self.ReceiveBeginPlay`
  (`self.Initiate`))

(event `self.ReceiveTick`
  (params (DeltaSeconds :type "Float (single-precision)"))
  (bind _direction (`self.GetCursorDirections`))
  (bind _newparam (`self.ShouldMove`))
  (if _newparam
    (`self.MoveCamera` _direction)))

(fn `GetCursorDirections`
  (returns (Direction :type "Vector Structure"))
  (bind (_returnvalue_x _returnvalue_y) (`KismetMathLibrary.BreakVector2D` (`WidgetLayoutLibrary.GetViewportSize`)))
  (bind (_locationx _locationy) (`PlayerController.GetMousePosition` (`self.Ref_PlayerController`)))
  (bind _value (`self.IsCursorThresholdCrossed` _locationx _returnvalue_x))
  (set `self.Direction_X` _value)
  (bind _value_2 (`self.IsCursorThresholdCrossed` _locationy _returnvalue_y))
  (set `self.Direction_Y` _value_2)
  (return (`KismetMathLibrary.MakeVector` (`self.Direction_X`) (`self.Direction_Y`))))

(fn `Initiate`
  (`PlayerController.SetViewTargetWithBlend` (`GameplayStatics.GetPlayerController` 0) self 0.0 "VTBlend_Linear" 0.0 false)
  (bind _asbp_controller_base (cast `/Game/Framework/Input/BP_ControllerBase` (`GameplayStatics.GetPlayerController` 0)))
  (set `self.Ref_PlayerController` _asbp_controller_base))

(fn `IsCursorThresholdCrossed`
  (params (CursorPosition :type "Float (double-precision)") (VIewportSize :type "Float (double-precision)"))
  (returns (Value :type "Float (double-precision)"))
  (locals (CursorValue :type "Float (double-precision)"))
  ; Gets cursor position, then checks whether this position is beyond the threshold at which camera should move. If so, sets the X / Y directions to the value that corresponds with how far over this threshold the cursor is.
  (if (`self.isCursorPositive` CursorPosition VIewportSize)
    (set `local.CursorValue` 1.0)
    (elif (not (`self.isCursorNegative` CursorPosition VIewportSize))
      (set `local.CursorValue` 0.0)
      (else
        (set `local.CursorValue` -1.0))))
  (return (`local.CursorValue`)))

(fn `MoveCamera`
  (params (Direction :type "Vector Structure"))
  (`SceneComponent.K2_AddRelativeLocation` (`self.DefaultSceneRoot`) (* Direction (`self.CameraSpeed`)) false false))

(fn `ShouldMove`
  (returns (NewParam :type Boolean))
  (bind (_direction_x _direction_y) (`KismetMathLibrary.BreakVector` (`/Game/Framework/Input/BP_ControllerBase.Direction` (`self.Ref_PlayerController`))))
  (return (or (and (== _direction_x 0.0) (== _direction_y 0.0)) (`self.CombineMovement`))))

(fn `UserConstructionScript`)
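; Base controller that turns Enhanced Input into camera control for the commander and spawns a Warrior unit for itself on BeginPlay.
; Move input is forwarded to the commander only when its own X/Y direction is zero or CombineMovement is enabled.
; Zoom input sets a clamped target arm length, which Tick eases the spring arm toward.
; A float curve maps normalized arm length to camera pitch, so the view tilts with zoom.
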(event `self.ReceiveBeginPlay`
  (`self.Initiate`)
  (`self.SpawnSquad`))

(event `EnhancedInput|/Game/Framework/Input/InputAction/IA_MoveCamera`
  (params (ActionValue :type "Vector2D Structure") (ElapsedSeconds :type "Float (double-precision)") (TriggeredSeconds :type "Float (double-precision)") (InputAction :type "InputAction Object Reference" :default "/Game/Framework/Input/InputAction/IA_MoveCamera.IA_MoveCamera"))
  ; Camera movement
  (:`Triggered`
    (`self.MoveCamera` ActionValue_X ActionValue_Y))
  (:`Canceled`
    (`self.OnMoveCameraEnd` :!label _label))
  (:`Completed`
    (goto _label)))

(event `EnhancedInput|/Game/Framework/Input/InputAction/IA_ZoomScroll`
  (params (ActionValue :type "Float (double-precision)") (ElapsedSeconds :type "Float (double-precision)") (TriggeredSeconds :type "Float (double-precision)") (InputAction :type "InputAction Object Reference" :default "/Game/Framework/Input/InputAction/IA_ZoomScroll.IA_ZoomScroll"))
  ; Scroll
  (:`Triggered`
    (`self.Scroll` ActionValue)))

(event `self.ReceiveTick`
  (params (DeltaSeconds :type "Float (single-precision)"))
  ; Scroll
  (`self.UpdateScroll` DeltaSeconds))

(fn `Initiate`
  ; Commander setup
  (bind _output_get (set `self.Commander Ref` (`/Game/Framework/CommonFunctions.CF_GetPlayer`)))
  ; Camera setup
  (bind _output_get_2 (set `self.TargetArmLength` (`SpringArmComponent.TargetArmLength` (`/Game/Framework/BP_Commander.SpringArm` _output_get))))
  (`self.RotateCameraAlongCurve` _output_get_2))

(fn `MoveCamera`
  (params (Direction_X :type "Float (double-precision)") (Direction_Y :type "Float (double-precision)"))
  (set `self.Direction` (`KismetMathLibrary.MakeVector` Direction_X Direction_Y))
  (bind _returnvalue (`self.ShouldMove`))
  (if _returnvalue
    (`/Game/Framework/BP_Commander.MoveCamera` (`self.Commander Ref`) (`self.Direction`))
    (`self.OnMoveCameraEnd`)))

(fn `RotateCameraAlongCurve`
  (params (Value :type "Float (double-precision)"))
  ; Takes current arm length, normalizes it between min/max and finds the corresponding rotation on CameraCurve
  (`SceneComponent.K2_SetRelativeRotation` (`/Game/Framework/BP_Commander.SpringArm` (`self.Commander Ref`)) (`KismetMathLibrary.MakeRotator` 0.0 (`CurveFloat.GetFloatValue` (`self.CameraCurve`) (`KismetMathLibrary.NormalizeToRange` Value (`self.MinScroll`) (`self.MaxScroll`)))) false false))

(fn `Scroll`
  (params (ActionValue :type "Float (double-precision)"))
  (set `self.TargetArmLength` (`KismetMathLibrary.FClamp` (+ (* ActionValue (`self.ScrollStrength`) -1.0) (`self.TargetArmLength`)) (`self.MinScroll`) (`self.MaxScroll`))))

(fn `ShouldMove`
  (returns (ReturnValue :type Boolean))
  (bind _commander_ref (`self.Commander Ref`))
  (return (or (and (== (`/Game/Framework/BP_Commander.Direction_X` _commander_ref) 0.0) (== (`/Game/Framework/BP_Commander.Direction_Y` _commander_ref) 0.0)) (`/Game/Framework/BP_Commander.CombineMovement` _commander_ref))))

(fn `SpawnSquad`
  (`UnitManager.SpawnUnit` (subsystem `UnitManager`) "Warrior" (0.0 0.0 0.0) self))

(fn `UpdateScroll`
  (params (DeltaTime :type "Float (double-precision)"))
  (bind _output_get (set `SpringArmComponent.TargetArmLength` (`KismetMathLibrary.FInterpTo` (`self.GetSpringArmLength`) (`self.TargetArmLength`) DeltaTime 1.0) (`/Game/Framework/BP_Commander.SpringArm` (`self.Commander Ref`))))
  (`self.RotateCameraAlongCurve` _output_get))

(fn `UserConstructionScript`)